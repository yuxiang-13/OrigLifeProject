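; BP_Car is a drivable Chaos wheeled vehicle with switchable in-car and rear cameras.
; Input axes feed throttle, brake and steering directly into the vehicle movement component.
; A FlipFlop on ChangeCamera toggles the active camera, while mouse turn input yaws both the SpringArm and RearCamera.
; BeginPlay caches the cast Chaos movement component, but the engine RPM sound update that reads it is unconnected and never runs.
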(event EventBeginPlay
  (bind _aschaos_wheeled_vehicle_movement_component (Utilities|Casting|CastToChaosWheeledVehicleMovementComponent (Variables|Default|GetVehicleMovementComponent)))
  (Variables|Default|SetAs%20Chaos%20Wheeled%20Vehicle%20Movement%20Component _aschaos_wheeled_vehicle_movement_component))

(event Collision|EventActorBeginOverlap
  (params (OtherActor :type Actor%20Object%20Reference)))

(event EventTick
  (params (DeltaSeconds :type Float%20%28single-precision%29)))

(event Input|ActionEvents|InputActionChangeCamera
  (params (Key :type Key%20Structure :default "None"))
  ;[1 1 1] 视角切换
  (:Pressed
    (Utilities|FlowControl|FlipFlop
      (:A
        (Components|Activation|SetActive (Variables|Default|GetCamera_InCar) true true)
        (Components|Activation|Deactivate (Variables|Default|GetRear_Camera)) ; 停用
      )
      (:B
        (Components|Activation|SetActive (Variables|Default|GetRear_Camera) true true)
        (Components|Activation|Deactivate (Variables|Default|GetCamera_InCar)) ; 停用
      ))))

(event Input|AxisEvents|InputAxisBrake
  (params (AxisValue :type Float%20%28single-precision%29))
  ;[1 1 1] 基本移动
  (Class|ChaosVehicleMovementComponent|SetBrakeInput (Variables|Default|GetVehicleMovementComponent) AxisValue))

(event Input|AxisEvents|InputAxisMoveRight
  (params (AxisValue :type Float%20%28single-precision%29))
  ;[1 1 1] 基本移动
  (Class|ChaosVehicleMovementComponent|SetSteeringInput (Variables|Default|GetVehicleMovementComponent) AxisValue))

(event Input|AxisEvents|InputAxisMoveForward
  (params (AxisValue :type Float%20%28single-precision%29))
  ;[1 1 1] 基本移动
  (Class|ChaosVehicleMovementComponent|SetThrottleInput (Variables|Default|GetVehicleMovementComponent) AxisValue))

(event Input|AxisEvents|InputAxisTurnRight/LeftMouse
  (params (AxisValue :type Float%20%28single-precision%29))
  (Transformation|AddRelativeRotation (Variables|Default|GetSpringArm) (Math|Rotator|MakeRotator 0.0 0.0 AxisValue) false false))

(fn ConstructionScript)